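; BP_Aranthian is a character Blueprint for a talkable Aranthian shown as a Paper2D sprite.
; Each tick it orients the sprite from the player controller's rotation, billboard style, and bobs it vertically with a cosine of game time.
; StartorContinueDialogue uses the player's DialogueComponent to advance an active dialogue or start one from this actor's DialogueID.
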(event EventBeginPlay)

(event Collision|EventActorBeginOverlap
  (params (OtherActor :type Actor%20Object%20Reference)))

(event EventTick
  (params (DeltaSeconds :type Float%20%28single-precision%29))
  (Transformation|AddLocalRotation (Variables|Default|GetPaperSprite) "0, 0, 0" false false)
  (Transformation|SetWorldRotation (Variables|Default|GetPaperSprite) (Math|Rotator|CombineRotators "-90.000000,0.000000,90.000000" (Transformation|GetActorRotation (Game|GetPlayerController 0))) false false)
  (Transformation|SetWorldLocation (Variables|Default|GetPaperSprite) (+ (Transformation|GetWorldLocation (Variables|Default|GetPaperSprite)) (Math|Vector|MakeVector 0.0 0.0 (* (Math|Trig|Cos(Radians) (Actor|GetGameTimeSinceCreation)) 0.5))) false false))

(event EventStartorContinueDialogue
  (params (Player :type OWH%20Character%20Object%20Reference))
  (bind _dialoguecomponent (Variables|/Script/OtherworldHunger.OWHCharacter|GetDialogueComponent Player))
  (if (Class|OWHDialogueComponent|IsinDialogue _dialoguecomponent)
    (Class|OWHDialogueComponent|GotoNextDialogue _dialoguecomponent)
    (else
      (Class|OWHDialogueComponent|StartDialogue _dialoguecomponent (Variables|Default|GetDialogueID)))))

(fn ConstructionScript)