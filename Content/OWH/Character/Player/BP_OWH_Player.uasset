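; Player character for OWH that ties together movement states, stamina, fall damage, the HUD, pause menu, dialogue and saved data.
; Walk/run toggling and damage use GAS abilities and effects, with loose tags and a timer gating stamina refill and exhaustion cooldown.
; BeginPlay creates the HUD and, if save loading is enabled, restores per-level transform and ingredient inventory, then binds DialogueComponent events that forward to the HUD's dialogue widget.
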(event Custom|OnStartDialogue
  (params (DialogueID :type String))
  (bind _widgethud (Variables|Default|GetWidgetHUD))
  (bind _wbp_dialogue (Variables|/Game/UI/WBP_MainHUD.WBP_MainHUD_C|GetWBP_Dialogue _widgethud))
  ;[0.9449 0.5425 1] Dialogue
  (Utilities|IsValid _widgethud
    (:Is%20Valid
      (Utilities|IsValid _wbp_dialogue
        (:Is%20Valid
          (Class|DialogueWidget|StartDialogue _wbp_dialogue DialogueID))))))

(event Custom|OnNextDialogue
  (params (DialogueID :type String) (Dialogue :type String))
  (bind _widgethud (Variables|Default|GetWidgetHUD))
  (bind _wbp_dialogue (Variables|/Game/UI/WBP_MainHUD.WBP_MainHUD_C|GetWBP_Dialogue _widgethud))
  ;[0.9449 0.5425 1] Dialogue
  (Utilities|IsValid _widgethud
    (:Is%20Valid
      (Utilities|IsValid _wbp_dialogue
        (:Is%20Valid
          (Class|DialogueWidget|NextDialogue _wbp_dialogue DialogueID Dialogue))))))

(event Custom|Cooldown
  ;[0.1337 1 0.8953] Walk/Run
  (Ability|GameplayEffect|AddLooseGameplayTags self (GameplayTags|MakeGameplayTagContainerfromTag "(TagName=\"Status.RefillStamina\")")))

(event Custom|EndStaminaTimer
  ;[0.1337 1 0.8953] Walk/Run
  (Utilities|Time|PauseTimerbyHandle (Variables|Default|GetStaminaCooldown))
  (Ability|GameplayEffect|RemoveLooseGameplayTags self (GameplayTags|MakeGameplayTagContainerfromTag "(TagName=\"Status.RefillStamina\")")))

(event Custom|OnEndDialogue
  (params (DialogueID :type String))
  (bind _widgethud (Variables|Default|GetWidgetHUD))
  (bind _wbp_dialogue (Variables|/Game/UI/WBP_MainHUD.WBP_MainHUD_C|GetWBP_Dialogue _widgethud))
  ;[0.9449 0.5425 1] Dialogue
  (Utilities|IsValid _widgethud
    (:Is%20Valid
      (Utilities|IsValid _wbp_dialogue
        (:Is%20Valid
          (Class|DialogueWidget|EndDialogue _wbp_dialogue DialogueID))))))

(event Custom|InitEffects
  ;[1 1 1] Initializer
  (GameplayEffects|ApplyGameplayEffectToSelf :self (Variables|Default|GetAbilitySystemComponent) :GameplayEffectClass "/Game/OWH/Abilities/GE_RefillStamina.GE_RefillStamina_C"))

(event Custom|ToWalking
  ;[0.1337 1 0.8953] Walk/Run
  (Abilities|TryActivateAbilitybyClass (Ability|GetAbilitySystemComponent 0) "/Game/OWH/Abilities/GPA_OWH_Walk.GPA_OWH_Walk_C" true)
  (CallFunction|RunStaminaTimer))

(event Custom|AddPlayerHUD
  ;[0.1527 0.3434 1] PlayerHUD
  (bind _returnvalue (UserInterface|CreateWidget "/Game/UI/WBP_MainHUD.WBP_MainHUD_C" (Game|GetPlayerController 0)))
  (bind _output_get (Variables|Default|SetWidgetHUD _returnvalue))
  (UserInterface|Viewport|AddtoViewport _returnvalue 0)
  (Class|OWHCharacter|SetPlayerHUD _output_get))

(event Custom|UpdateHealth
  ;[1 0.4974 0.6361] HealthRef
  (Variables|Default|SetHealthRef (.basevalue (Variables|/Script/OtherworldHunger.BasicAttributeSet|GetHealth (Variables|Default|GetAttributes)))))

(event Custom|UpdateStamina
  (bind _returnvalue (GameplayTags|MakeGameplayTagContainerfromTag "(TagName=\"Status.StaminaCooldown\")"))
  (bind _returnvalue_2 (Ability|GetAbilitySystemComponent 0))
  (bind _self self)
  (bind _attributes (Variables|Default|GetAttributes))
  (bind _tagcontainer (GameplayTags|GetOwnedGameplayTags _returnvalue_2 :!class /Script/GameplayTags.GameplayTagAssetInterface))
  (bind _stamina (Variables|/Script/OtherworldHunger.BasicAttributeSet|GetStamina _attributes))
  (bind _returnvalue_3 (GameplayTags|HasTag _tagcontainer "(TagName=\"Status.StaminaCooldown\")"))
  ;[0.1337 1 0.8953] StaminaRef
  (Variables|Default|SetStaminaRef (.basevalue _stamina))
  ;[0.2374 0.6506 0.8099] StaminaCooldown
  (if (== (.basevalue _stamina) 0.0)
    (if (not _returnvalue_3)
      (CallFunction|ToWalking)
      (Ability|GameplayEffect|AddLooseGameplayTags _self _returnvalue)
      (Ability|SendGameplayEventtoActor _self "(TagName=\"Status.StaminaCooldown\")"))
    (elif _returnvalue_3
      (if (== (.basevalue _stamina) 1e+02)
        (Ability|GameplayEffect|RemoveLooseGameplayTags _self _returnvalue)
        (Variables|/Script/Engine.CharacterMovementComponent|SetMaxWalkSpeed (Variables|Character|GetCharacterMovement) 5e+02)))))

(event Custom|RunStaminaTimer
  ;[0.1337 1 0.8953] Walk/Run
  (bind _returnvalue (Utilities|Time|SetTimerbyEvent (delegate Custom|Cooldown) 2.5))
  (Variables|Default|SetStaminaCooldown _returnvalue))

(event Input|EnhancedActionEvents|EnhancedInputActionIA_OWH_Walk
  (params (ActionValue :type Boolean) (ElapsedSeconds :type Float%20%28double-precision%29) (TriggeredSeconds :type Float%20%28double-precision%29) (InputAction :type Input%20Action%20Object%20Reference :default "/Game/OWH/Input/IA_OWH_Walk.IA_OWH_Walk"))
  (bind _returnvalue (Ability|GetAbilitySystemComponent 0))
  (bind _tagcontainer (GameplayTags|GetOwnedGameplayTags _returnvalue :!class /Script/GameplayTags.GameplayTagAssetInterface))
  ;[0.1337 1 0.8953] Walk/Run
  (if (not (Variables|Default|GetbIsClimbing))
    (if (not (GameplayTags|HasTag _tagcontainer "(TagName=\"Status.StaminaCooldown\")"))
      (if (GameplayTags|HasTag _tagcontainer "(TagName=\"Status.IsRunning\")")
        (Abilities|TryActivateAbilitybyClass _returnvalue "/Game/OWH/Abilities/GPA_OWH_Walk.GPA_OWH_Walk_C" true)
        (CallFunction|RunStaminaTimer)
        (else
          (Abilities|TryActivateAbilitybyClass _returnvalue "/Game/OWH/Abilities/GPA_OWH_Run.GPA_OWH_Run_C" true)
          (CallFunction|EndStaminaTimer))))))

(event EventBeginPlay
  ;[0.1745 0.1745 0.1745] Player Save Data
  (CallFunction|InitEffects)
  (CallFunction|AddPlayerHUD)
  (if (Variables|Default|GetLoadPlayerSave) ; Player saved data can be disabled for testing
    (bind _savegamedata (Class|BPISaveGame|GetGameData(Message) (Game|GetGameInstance)))
    (Utilities|IsValid _savegamedata
      (:Is%20Valid
        (bind _returnvalue (Game|GetCurrentLevelName true))
        (CallFunction|UsePlayerSave (Variables|/Game/Blueprints/SavedGameData/BP_SaveGame.BP_SaveGame_C|GetPlayerSave _savegamedata) _returnvalue)
        (CallFunction|BindDialogueEvents)))))

(event EventOnLanded
  (params (Hit :type Hit%20Result%20Structure%20%28by%20ref%29))
  (bind _returnvalue (Pawn|GetMovementComponent))
  (bind _returnvalue_2 (Ability|GetAbilitySystemComponent 0))
  (bind _velocity (Variables|/Script/Engine.MovementComponent|GetVelocity _returnvalue))
  ;[1 0.4974 0.6361] FallDamage
  (if (< (.z _velocity) -1.6e+03)
    (bind _returnvalue_3 (Class|OWHCharacter|FallDamage (.z _velocity)))
    (bind _returnvalue_4 (Ability|GameplayEffect|AssignTagSetbyCallerMagnitude (GameplayEffects|MakeOutgoingSpec :self _returnvalue_2 :GameplayEffectClass "/Game/OWH/Abilities/GE_TakeDamage.GE_TakeDamage_C") "(TagName=\"Calculate.Damage\")" _returnvalue_3))
    (GameplayEffects|ApplyGameplayEffectSpecToSelf _returnvalue_2 _returnvalue_4)
    (CallFunction|UpdateHealth)))

(event EventTick
  (params (DeltaSeconds :type Float%20%28single-precision%29))
  ;[1 1 1] Tick
  (CallFunction|UpdateStamina))

(event Input|KeyboardEvents|Escape
  (params (Key :type Key%20Structure :default "None"))
  ;[1 1 1] PauseMenu
  (:Pressed
    (Default|PushWidget (Variables|Default|GetWidgetHUD) "/Game/UI/WBP_PauseMenu.WBP_PauseMenu_C")))

(fn ConstructionScript)

(fn GetPlayerSave
  (bind _savegamedata (Class|BPISaveGame|GetGameData(Message) (Game|GetGameInstance)))
  (bind _returnvalue (Game|GetCurrentLevelName true))
  (Utilities|Map|Add (.Transform (Utilities|Struct|BreakS_PlayerData (Variables|/Game/Blueprints/SavedGameData/BP_SaveGame.BP_SaveGame_C|GetPlayerSave _savegamedata))) _returnvalue (Transformation|GetActorTransform))
  (Utilities|Map|Add (.ControlRotation (Utilities|Struct|BreakS_PlayerData (Variables|/Game/Blueprints/SavedGameData/BP_SaveGame.BP_SaveGame_C|GetPlayerSave _savegamedata))) _returnvalue (Pawn|GetControlRotation :!class /Script/Engine.Pawn))
  (return (Utilities|Struct|MakeS_PlayerData (.Transform (Utilities|Struct|BreakS_PlayerData (Variables|/Game/Blueprints/SavedGameData/BP_SaveGame.BP_SaveGame_C|GetPlayerSave _savegamedata))) (.ControlRotation (Utilities|Struct|BreakS_PlayerData (Variables|/Game/Blueprints/SavedGameData/BP_SaveGame.BP_SaveGame_C|GetPlayerSave _savegamedata))) (Variables|/Script/OtherworldHunger.OWHCharacterInventory|GetIngredientMap (Variables|Default|GetCharacterInventory)))))

(fn UsePlayerSave
  (params (S_PlayerData :type S%20Player%20Data%20Structure) (Level :type String))
  (bind _value (Utilities|Map|Find (.transform S_PlayerData) Level))
  (bind _characterinventory (Variables|Default|GetCharacterInventory))
  (if (not (== _value (Math|Transform|MakeTransform "0, 0, 0")))
    (Transformation|SetActorTransform _value)
    (Pawn|SetControlRotation (Pawn|GetController) (.Value (Utilities|Map|Find (.controlrotation S_PlayerData) Level)))
    (Variables|/Script/OtherworldHunger.OWHCharacterInventory|SetIngredientMap _characterinventory (.inventory S_PlayerData))
    (Class|OWHCharacterInventory|DisplayIngredients _characterinventory)))

(fn BindDialogueEvents
  (bind _dialoguecomponent (Variables|Default|GetDialogueComponent))
  (Utilities|IsValid _dialoguecomponent
    (:Is%20Valid
      (EventDispatchers|BindEventtoOnStartDialogue _dialoguecomponent (EventDispatchers|CreateEvent :!event Custom|OnStartDialogue))
      (EventDispatchers|BindEventtoOnNextDialogue _dialoguecomponent (EventDispatchers|CreateEvent :!event Custom|OnNextDialogue))
      (EventDispatchers|BindEventtoOnEndDialogue _dialoguecomponent (EventDispatchers|CreateEvent :!event Custom|OnEndDialogue)))))

(fn TakeDamage
  (bind _self self)
  (bind _returnvalue (Ability|GetAbilitySystemComponent _self))
  (bind _returnvalue_2 (Ability|GameplayEffect|AssignTagSetbyCallerMagnitude (GameplayEffects|MakeOutgoingSpec :self _returnvalue :GameplayEffectClass "/Game/OWH/Abilities/GE_TakeDamage.GE_TakeDamage_C") "(TagName=\"Calculate.Damage\")" -3e+01))
  (GameplayEffects|ApplyGameplayEffectSpecToSelf _returnvalue _returnvalue_2))