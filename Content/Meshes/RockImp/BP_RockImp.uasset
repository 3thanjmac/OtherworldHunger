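; Rock Imp enemy character that chases and melee-attacks the player, driven by an Idle/Chase/Attack state switch on Tick.
; PawnSensing starts the chase, which moves to Attack within range or Idle when the player escapes.
; Attacking stops movement, turns smoothly toward the player and plays a charge montage.
; Weapon overlaps apply damage, while taking damage forces Attack, reduces Health and destroys the imp shortly after it reaches zero.
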(event OnSeePawn(PawnSensing)
  (params (Pawn :type Pawn%20Object%20Reference))
  ;[1 1 1] On See Pawn
  (Utilities|Casting|CastToBP_OWH_Player Pawn)
  (Variables|Default|SetEnemyStates "NewEnumerator1"))

(event OnComponentBeginOverlap(WeaponCollider)
  (params (OverlappedComponent :type Primitive%20Component%20Object%20Reference) (OtherActor :type Actor%20Object%20Reference) (OtherComp :type Primitive%20Component%20Object%20Reference) (OtherBodyIndex :type Integer) (bFromSweep :type Boolean) (SweepResult :type Hit%20Result%20Structure%20%28by%20ref%29))
  (if (!= OtherActor self)
    (Game|Damage|ApplyDamage OtherActor (Variables|Default|GetWeaponDamage) 0 0)
    (if (== OtherActor (Variables|Default|GetPlayer))
      (CallFunction|EndCollision (Variables|Default|GetWeaponCollider)))))

(event EventBeginPlay
  ;[1 1 1] BeginPlay
  (bind _asbp_owh_player (Utilities|Casting|CastToBP_OWH_Player (Game|GetPlayerCharacter 0)))
  (Variables|Default|SetPlayer _asbp_owh_player))

(event Collision|EventActorBeginOverlap
  (params (OtherActor :type Actor%20Object%20Reference)))

(event EventTick
  (params (DeltaSeconds :type Float%20%28single-precision%29))
  (bind _player (Variables|Default|GetPlayer))
  (bind _returnvalue (Transformation|GetHorizontalDistanceTo _player))
  ;[1 1 1] Tick
  (switch Utilities|FlowControl|Switch|SwitchonEnemyStates (Variables|Default|GetEnemyStates)
    (:NewEnumerator1
      (AI|AIMoveTo self (Transformation|GetActorLocation (Variables|Default|GetPlayer)) 0 5.0 false
        (:then
          (if (<= _returnvalue (Variables|Default|GetAttackRange))
            (Variables|Default|SetEnemyStates "NewEnumerator2")
            (elif (>= _returnvalue (Variables|Default|GetRangeToLoseInterest))
              (Variables|Default|SetEnemyStates "NewEnumerator0"))))))
    (:NewEnumerator2
      (Components|Movement|StopMovementImmediately (Variables|Character|GetCharacterMovement))
      (CallFunction|FaceTarget DeltaSeconds)
      (if (not (Variables|Default|GetIsAttacking))
        (Variables|Default|SetIsAttacking true)
        (Animation|PlayAnimMontage "/Game/Meshes/RockImp/Animations/AM_RockImpAttacks2.AM_RockImpAttacks2" 1.0 "ChargeAttack")))))

(event Game|Damage|EventAnyDamage
  (params (Damage :type Float%20%28single-precision%29) (DamageType :type Damage%20Type%20Object%20Reference) (InstigatedBy :type Controller%20Object%20Reference) (DamageCauser :type Actor%20Object%20Reference))
  (Variables|Default|SetEnemyStates "NewEnumerator2")
  (bind _output_get (Variables|Default|SetHealth (- (Variables|Default|GetHealth) Damage)))
  (Development|PrintString (Utilities|String|ToString(Float) _output_get))
  (if (<= _output_get 0.0)
    (Utilities|FlowControl|Delay 0.3)
    (Actor|DestroyActor)))

(fn ConstructionScript)

(fn StartCollision
  (params (Box%20Collider :type Box%20Component%20Object%20Reference))
  (Collision|SetCollisionProfileName Box%20Collider "OverlapAllDynamic" true :!class /Script/Engine.PrimitiveComponent))

(fn EndCollision
  (params (BoxCollider :type Box%20Component%20Object%20Reference))
  (Collision|SetCollisionProfileName BoxCollider "OverlapAllDynamic" true :!class /Script/Engine.PrimitiveComponent))

(fn FaceTarget
  (params (DeltaTime :type Float%20%28double-precision%29))
  (Transformation|SetActorRotation (Math|Interpolation|RInterpTo (Transformation|GetActorRotation) (Math|Rotator|FindLookatRotation (Transformation|GetActorLocation) (Transformation|GetActorLocation (Variables|Default|GetPlayer))) DeltaTime (Variables|Default|GetTurnSpeed))))