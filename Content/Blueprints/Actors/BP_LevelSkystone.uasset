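; BP_LevelSkystone is a level skystone actor that reveals a text label and animates a plane's opacity while something overlaps it.
; BeginPlay creates a dynamic material instance for the plane and hides the text.
; Overlap begin shows the text and plays a timeline driving the OpacityScalar parameter, and overlap end hides the text and reverses it.
; The overlapping actor is not filtered.
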(event EventBeginPlay
  ;[1 1 1] Dynamic Material
  (bind _returnvalue (Rendering|Material|CreateDynamicMaterialInstance (Rendering|Material|GetMaterial (Variables|Default|GetPlane) 0) "None" "None" :!class /Script/Engine.KismetMaterialLibrary))
  (bind _output_get (Variables|Default|SetPlaneMaterial _returnvalue))
  (Rendering|Material|SetMaterial (Variables|Default|GetPlane) 0 _output_get)
  (Rendering|SetVisibility (Variables|Default|GetText) false false))

(event Collision|EventActorBeginOverlap
  (params (OtherActor :type Actor%20Object%20Reference))
  (Rendering|SetVisibility (Variables|Default|GetText) true false)
  (bind _lerp (Timeline|LerpMaterial Play)
    (:Update
      (Rendering|Material|SetScalarParameterValue (Variables|Default|GetPlaneMaterial) "OpacityScalar" _lerp :!class /Script/Engine.MaterialInstanceDynamic))))

(event Collision|EventActorEndOverlap
  (params (OtherActor :type Actor%20Object%20Reference))
  (Rendering|SetVisibility (Variables|Default|GetText) false false)
  (bind _lerp (Timeline|LerpMaterial Reverse)
    (:Update
      (Rendering|Material|SetScalarParameterValue (Variables|Default|GetPlaneMaterial) "OpacityScalar" _lerp :!class /Script/Engine.MaterialInstanceDynamic))))

(fn ConstructionScript)