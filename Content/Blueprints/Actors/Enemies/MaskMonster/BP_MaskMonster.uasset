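; BP_MaskMonster is a melee enemy that attacks while the player is inside its detection box and is destroyed when Health runs out.
; Tick starts the attack montage when CanAttack allows, clearing that flag without resetting it here, and also checks Health.
; The attack hitbox damages other overlapping actors, with functions to toggle its collision.
; Incoming damage plays a sound, lowers Health and prints it; FacePlayer is an empty stub.
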(event OnComponentBeginOverlap(PlayerDetectionBox)
  (params (OverlappedComponent :type Primitive%20Component%20Object%20Reference) (OtherActor :type Actor%20Object%20Reference) (OtherComp :type Primitive%20Component%20Object%20Reference) (OtherBodyIndex :type Integer) (bFromSweep :type Boolean) (SweepResult :type Hit%20Result%20Structure%20%28by%20ref%29))
  (Utilities|Casting|CastToBP_OWH_Player OtherActor)
  (Variables|Default|SetShouldAttackPlayer true))

(event OnComponentBeginOverlap(AttackHitBox)
  (params (OverlappedComponent :type Primitive%20Component%20Object%20Reference) (OtherActor :type Actor%20Object%20Reference) (OtherComp :type Primitive%20Component%20Object%20Reference) (OtherBodyIndex :type Integer) (bFromSweep :type Boolean) (SweepResult :type Hit%20Result%20Structure%20%28by%20ref%29))
  (if (not (== OtherActor self))
    (Game|Damage|ApplyDamage OtherActor (Variables|Default|GetBaseDamage) 0 0)))

(event OnComponentEndOverlap(PlayerDetectionBox)
  (params (OverlappedComponent :type Primitive%20Component%20Object%20Reference) (OtherActor :type Actor%20Object%20Reference) (OtherComp :type Primitive%20Component%20Object%20Reference) (OtherBodyIndex :type Integer))
  (Utilities|Casting|CastToBP_OWH_Player OtherActor)
  (Variables|Default|SetShouldAttackPlayer false))

(event EventBeginPlay)

(event Collision|EventActorBeginOverlap
  (params (OtherActor :type Actor%20Object%20Reference)))

(event EventTick
  (params (DeltaSeconds :type Float%20%28single-precision%29))
  (Utilities|FlowControl|Sequence
    (:then_0
      (if (Variables|Default|GetShouldAttackPlayer)
        (if (Variables|Default|GetCanAttack)
          (Variables|Default|SetCanAttack false)
          (Animation|Montage|PlayMontage (Variables|Default|GetSkeletalMesh) "/Game/Blueprints/Actors/Enemies/MaskMonster/Am_MaskMonster.Am_MaskMonster" 1.0 0.0 "Attack1"))))
    (:then_1
      (if (<= (Variables|Default|GetHealth) 0.0)
        (Actor|DestroyActor)))))

(event Game|Damage|EventAnyDamage
  (params (Damage :type Float%20%28single-precision%29) (DamageType :type Damage%20Type%20Object%20Reference) (InstigatedBy :type Controller%20Object%20Reference) (DamageCauser :type Actor%20Object%20Reference))
  (Audio|PlaySoundatLocation "/Engine/VREditor/Sounds/VR_teleport.VR_teleport" (Transformation|GetActorLocation) "0, 0, 0" 0.75 1.0 0.0 0 0 0 0)
  (bind _output_get (Variables|Default|SetHealth (- (Variables|Default|GetHealth) Damage)))
  (Development|PrintString (Utilities|String|ToString(Float) _output_get)))

(fn ConstructionScript)

(fn EnableCollision
  (Collision|SetCollisionProfileName (Variables|Default|GetAttackHitBox) "OverlapAllDynamic" true :!class /Script/Engine.PrimitiveComponent))

(fn DisableCollision
  (Collision|SetCollisionEnabled (Variables|Default|GetAttackHitBox) "NoCollision"))

(fn FacePlayer
  (params (DeltaTime :type Float%20%28double-precision%29)))