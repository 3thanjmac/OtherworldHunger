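; BP_PlantMonster is a plant trap enemy that bites when an actor overlaps it.
; After a short delay it sets IsBiting, then a timer fires Release to clear it.
; DoDamage and TakeDamage both apply a fixed negative base damage to the first BP_OWH_Player overlapping the capsule, ignoring TakeDamage's Damage input.
; Neither is called within this Blueprint, so biting and damage are not linked here.
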(event Custom|Release
  (Variables|Default|SetbIsBiting false))

(event Collision|EventActorBeginOverlap
  (params (OtherActor :type Actor%20Object%20Reference))
  (Utilities|FlowControl|Delay 1.5)
  (Variables|Default|SetbIsBiting true)
  (Utilities|Time|SetTimerbyEvent (delegate Custom|Release) 5.0))

(event EventDoDamage
  (params (Damage :type Float%20%28double-precision%29))
  (Game|Damage|ApplyDamage (Utilities|Array|Get(acopy) (Collision|GetOverlappingActors (Variables|Default|GetCapsule) "/Game/OWH/Character/Player/BP_OWH_Player.BP_OWH_Player_C" :!class /Script/Engine.PrimitiveComponent)) -3e+01 0 0))

(fn ConstructionScript)

(fn TakeDamage
  (params (Damage :type Float%20%28double-precision%29))
  (Game|Damage|ApplyDamage (Utilities|Array|Get(acopy) (Collision|GetOverlappingActors (Variables|Default|GetCapsule) "/Game/OWH/Character/Player/BP_OWH_Player.BP_OWH_Player_C" :!class /Script/Engine.PrimitiveComponent)) -3e+01 0 0))